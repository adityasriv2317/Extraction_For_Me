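; Base pickup actor for a world weapon that the main character can take.
; Overlapping its interaction sphere shows the character a pickup prompt with the name and icon read from the weapon class defaults, and leaving hides it.
; Interacting has the character spawn that weapon in hand and hide the prompt, then the pickup destroys itself.
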(event `/Game/Blueprints/Interfaces/BPI_Weapons.Interact_WithGun`
  (params (MainPlayer :type "/Game/Blueprints/BP_MainCharacter Object Reference"))
  (`/Game/Blueprints/BP_MainCharacter.Spawn Weapon in_Hand` MainPlayer (`self.Weapon`))
  (`/Game/Blueprints/BP_MainCharacter.Hide_Weapon_Pickup_Prompt` MainPlayer)
  (`self.K2_DestroyActor`))

(event `self.InteractionSphere.OnComponentBeginOverlap`
  (params (OverlappedComponent :type "PrimitiveComponent Object Reference") (OtherActor :type "Actor Object Reference") (OtherComp :type "PrimitiveComponent Object Reference") (OtherBodyIndex :type Integer) (bFromSweep :type Boolean) (SweepResult :type "HitResult Structure (by ref)"))
  (bind (_emitterparticle _weaponpickup _reloadtime _weaponname _weapondamage _firerate _weaponicon) (defaults `Object` (`self.Weapon`)))
  (bind _asbp_main_character (cast `/Game/Blueprints/BP_MainCharacter` OtherActor))
  (`/Game/Blueprints/BP_MainCharacter.Show_Weapon_Pickup_Widget` _asbp_main_character _weaponicon _weaponname))

(event `self.InteractionSphere.OnComponentEndOverlap`
  (params (OverlappedComponent :type "PrimitiveComponent Object Reference") (OtherActor :type "Actor Object Reference") (OtherComp :type "PrimitiveComponent Object Reference") (OtherBodyIndex :type Integer))
  (bind _asbp_main_character (cast `/Game/Blueprints/BP_MainCharacter` OtherActor))
  (`/Game/Blueprints/BP_MainCharacter.Hide_Weapon_Pickup_Prompt` _asbp_main_character))

(fn `UserConstructionScript`)