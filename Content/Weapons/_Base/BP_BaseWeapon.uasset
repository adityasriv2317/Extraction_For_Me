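; BP_BaseWeapon is a base weapon Blueprint providing shared hitscan firing logic, with empty Shoot and EndShoot events.
; Create_LineTrace plays a muzzle effect on the Arrow, then runs a multi-object trace forward over a given range against Pawn and WorldStatic.
; Each hit receives WeaponDamage and an impact particle from SpawnHitParticle, chosen by the actor's first tag: electric for Enemy, brick otherwise.
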(event `Shoot`)

(event `EndShoot`)

(event `Create_LineTrace`
  (params (Range :type "Float (double-precision)"))
  (bind _arrow (`self.Arrow`))
  (bind _returnvalue (`SceneComponent.K2_GetComponentLocation` _arrow))
  (`GameplayStatics.SpawnEmitterAttached` "/Game/Realistic_Starter_VFX_Pack_Vol2/Particles/Explosion/P_Explosion_Big_A.P_Explosion_Big_A" _arrow "None" (0.0 0.0 0.0) (struct) (0.03 0.03 0.03))
  (bind (_outhits _returnvalue_2) (`KismetSystemLibrary.LineTraceMultiForObjects` _returnvalue (+ _returnvalue (* (`KismetMathLibrary.GetForwardVector` (`SceneComponent.K2_GetComponentRotation` _arrow)) Range)) (`|MakeArray` "ObjectTypeQuery3" "ObjectTypeQuery1" :!type "EObjectTypeQuery Enum")))
  (if _returnvalue_2
    (for _array_element _outhits
      (bind (_bblockinghit _binitialoverlap _time _distance _location _impactpoint _normal _impactnormal _physmat _hitactor) (`GameplayStatics.BreakHitResult` _array_element))
      (`self.Spawn HitParticle` (`|GetArrayItem` (`Actor.Tags` _hitactor)) _location)
      (`GameplayStatics.ApplyDamage` _hitactor (`self.WeaponDamage`)))))

(event `Spawn HitParticle`
  (params (TagName :type Name) (Location :type "Vector Structure"))
  (switch `name` TagName
    (:`Default`
      (set `self.EmitterParticle` "/Game/Realistic_Starter_VFX_Pack_Vol2/Particles/Hit/P_Brick.P_Brick"))
    (:`Enemy`
      (set `self.EmitterParticle` "/Game/Realistic_Starter_VFX_Pack_Vol2/Particles/Destruction/P_Destruction_Electric.P_Destruction_Electric")))
  (`GameplayStatics.SpawnEmitterAtLocation` (`self.EmitterParticle`) Location (struct) (0.5 0.5 0.5)))

(fn `UserConstructionScript`)